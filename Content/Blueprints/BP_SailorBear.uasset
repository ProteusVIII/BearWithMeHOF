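; BP_SailorBear is an interactable bear NPC that responds when the player brings it wood.
; A sphere overlap registers it as the player's InteractableObject and shows a prompt widget, gated by a DoOnce that resets on exit.
; Overlap creates WBP_RegularBearFish but checks for and removes WBP_SailorBearWood, so that prompt is never cleared here.
; Interact only prints a placeholder message when the in-range player has wood.
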(event OnComponentBeginOverlap(Sphere)
  (params (OverlappedComponent :type Primitive%20Component%20Object%20Reference) (OtherActor :type Actor%20Object%20Reference) (OtherComp :type Primitive%20Component%20Object%20Reference) (OtherBodyIndex :type Integer) (bFromSweep :type Boolean) (SweepResult :type Hit%20Result%20Structure%20%28by%20ref%29))
  (bind _asbp_player_character (Utilities|Casting|CastToBP_PlayerCharacter OtherActor))
  (Utilities|FlowControl|DoOnce false
    (:Completed
      (Variables|/Game/Blueprints/BP_PlayerCharacter.BP_PlayerCharacter_C|SetInteractableObject _asbp_player_character self)
      (Variables|Default|SetPlayerInRange? true)
      (bind _foundwidgets (Widget|GetAllWidgetsOfClass "/Game/Blueprints/Interaction/WBP_SailorBearWood.WBP_SailorBearWood_C" true))
      (Utilities|IsValid (Utilities|Array|Get(acopy) _foundwidgets)
        (:Is%20Not%20Valid
          (bind _returnvalue (UserInterface|CreateWidget "/Game/Blueprints/Interaction/WBP_RegularBearFish.WBP_RegularBearFish_C"))
          (UserInterface|Viewport|AddtoViewport _returnvalue 0))))))

(event OnComponentEndOverlap(Sphere)
  (params (OverlappedComponent :type Primitive%20Component%20Object%20Reference) (OtherActor :type Actor%20Object%20Reference) (OtherComp :type Primitive%20Component%20Object%20Reference) (OtherBodyIndex :type Integer))
  (bind _asbp_player_character (Utilities|Casting|CastToBP_PlayerCharacter OtherActor))
  (Utilities|FlowControl|Sequence
    (:then_0
      (Variables|/Game/Blueprints/BP_PlayerCharacter.BP_PlayerCharacter_C|SetInteractableObject _asbp_player_character 0)
      (Variables|Default|SetPlayerInRange? false)
      (bind _foundwidgets (Widget|GetAllWidgetsOfClass "/Game/Blueprints/Interaction/WBP_SailorBearWood.WBP_SailorBearWood_C" true))
      (for _array_element _foundwidgets
        (Widget|RemovefromParent _array_element)))
    (:then_1
      (Utilities|FlowControl|DoOnce false) ; enters at Reset
    )))

(event EventBeginPlay)

(event Collision|EventActorBeginOverlap
  (params (OtherActor :type Actor%20Object%20Reference)))

(event EventTick
  (params (DeltaSeconds :type Float%20%28single-precision%29)))

(event EventInteract
  (if (Variables|Default|GetPlayerInRange?)
    (if (Variables|/Game/Blueprints/BP_PlayerCharacter.BP_PlayerCharacter_C|GetHasWood (stale OnComponentBeginOverlap(Sphere) _asbp_player_character))
      (Development|PrintString "Nice Wood There"))))

(fn ConstructionScript)