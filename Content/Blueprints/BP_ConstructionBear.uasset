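; Construction bear NPC that accepts a pastry from the player as lunch, then moves to a new spot.
; Sphere overlap registers it as the player's interactable and shows a prompt widget until the player leaves.
; Interacting with a pastry sets GaveConstructionLunch once and removes the widget.
; Inside that removal loop, it starts a level sequence and timeline-driven turns around a move to a hard-coded location.
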(event OnComponentBeginOverlap(Sphere)
  (params (OverlappedComponent :type Primitive%20Component%20Object%20Reference) (OtherActor :type Actor%20Object%20Reference) (OtherComp :type Primitive%20Component%20Object%20Reference) (OtherBodyIndex :type Integer) (bFromSweep :type Boolean) (SweepResult :type Hit%20Result%20Structure%20%28by%20ref%29))
  (bind _asbp_player_character (Utilities|Casting|CastToBP_PlayerCharacter OtherActor))
  (if (not (Variables|Default|GetHasInteracted?))
    (Utilities|FlowControl|DoOnce false
      (:Completed
        (Variables|/Game/Blueprints/BP_PlayerCharacter.BP_PlayerCharacter_C|SetInteractableObject _asbp_player_character self)
        (Variables|Default|SetPlayerInRange? true)
        (bind _foundwidgets (Widget|GetAllWidgetsOfClass "/Game/Blueprints/Interaction/WBP_ConstructionBear.WBP_ConstructionBear_C" true))
        (Utilities|IsValid (Utilities|Array|Get(acopy) _foundwidgets)
          (:Is%20Not%20Valid
            (bind _returnvalue (UserInterface|CreateWidget "/Game/Blueprints/Interaction/WBP_ConstructionBear.WBP_ConstructionBear_C"))
            (UserInterface|Viewport|AddtoViewport _returnvalue 0)))))))

(event OnComponentEndOverlap(Sphere)
  (params (OverlappedComponent :type Primitive%20Component%20Object%20Reference) (OtherActor :type Actor%20Object%20Reference) (OtherComp :type Primitive%20Component%20Object%20Reference) (OtherBodyIndex :type Integer))
  (bind _asbp_player_character (Utilities|Casting|CastToBP_PlayerCharacter OtherActor))
  (Utilities|FlowControl|Sequence
    (:then_0
      (Variables|/Game/Blueprints/BP_PlayerCharacter.BP_PlayerCharacter_C|SetInteractableObject _asbp_player_character 0)
      (Variables|Default|SetPlayerInRange? false)
      (bind _foundwidgets (Widget|GetAllWidgetsOfClass "/Game/Blueprints/Interaction/WBP_ConstructionBear.WBP_ConstructionBear_C" true))
      (for _array_element _foundwidgets
        (Widget|RemovefromParent _array_element)))
    (:then_1
      (Utilities|FlowControl|DoOnce false) ; enters at Reset
    )))

(event EventBeginPlay
  (Variables|Default|SetSleeping? false))

(event Collision|EventActorBeginOverlap
  (params (OtherActor :type Actor%20Object%20Reference)))

(event EventTick
  (params (DeltaSeconds :type Float%20%28single-precision%29)))

(event EventInteract
  (if (Variables|Default|GetPlayerInRange?)
    (if (Variables|/Game/Blueprints/BP_PlayerCharacter.BP_PlayerCharacter_C|GetHasPastry (stale OnComponentBeginOverlap(Sphere) _asbp_player_character))
      (Utilities|FlowControl|DoOnce false
        (:Completed
          (Variables|/Game/Blueprints/BP_PlayerCharacter.BP_PlayerCharacter_C|SetGaveConstructionLunch (stale OnComponentBeginOverlap(Sphere) _asbp_player_character) true)
          (Variables|Default|SetHasInteracted? true)
          (bind _foundwidgets (Widget|GetAllWidgetsOfClass "/Game/Blueprints/Interaction/WBP_ConstructionBear.WBP_ConstructionBear_C" true))
          (for _array_element _foundwidgets
            (Widget|RemovefromParent _array_element)
            (bind _outactor (Sequencer|Player|CreateLevelSequencePlayer "/Game/LS_ConstructionBear.LS_ConstructionBear"))
            (Sequencer|Player|Play (Variables|/Script/LevelSequence.LevelSequenceActor|GetSequencePlayer _outactor) :!class /Script/MovieScene.MovieSceneSequencePlayer)
            (bind _alpha (Timeline|Timeline PlayFromStart)
              (:Update
                (Transformation|SetWorldRotation (Variables|Collision|GetCapsuleComponent) (Math|Rotator|Lerp(Rotator) (Transformation|GetWorldRotation (Variables|Collision|GetCapsuleComponent)) "0.000000,-160.000000,0.000000" _alpha) false false))
              (:Finished
                (Components|MoveComponentTo (Variables|Collision|GetCapsuleComponent) "1972.115665,-10302.115665,0.000000" "0.000000,-160.000000,0.000000" false false 1.0 false)
                (Utilities|FlowControl|Delay 1.0)
                (bind _alpha_2 (Timeline|Timeline_0 PlayFromStart)
                  (:Update
                    (Transformation|SetWorldRotation (Variables|Collision|GetCapsuleComponent) (Math|Rotator|Lerp(Rotator) (Transformation|GetWorldRotation (Variables|Collision|GetCapsuleComponent)) "0.000000,30.000000,0.000000" _alpha_2) false false)))))))))))

(fn ConstructionScript)